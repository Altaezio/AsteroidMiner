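; BP_ChunkSpawner is an actor that fills a three-dimensional grid with BP_Chunk actors when play begins.
; Nested loops over Width, Height and Length, mapped to X, Y and Z, place each chunk at its index multiplied by Chunksize.
; Positions are absolute world coordinates independent of the spawner's location, and every chunk spawns regardless of collision, with no rotation and unit scale.
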(event `self.ReceiveBeginPlay`
  (bind _chunksize (`self.chunksize`))
  (for _index (range (+ (`self.width`) 1))
    (for _index_2 (range (+ (`self.height`) 1))
      (for _index_3 (range (+ (`self.length`) 1))
        (`|SpawnActorFromClass` "/Game/Blueprints/BP_Chunk.BP_Chunk_C" (`KismetMathLibrary.MakeTransform` (`KismetMathLibrary.MakeVector` (`KismetMathLibrary.Conv_IntToDouble` (* _index _chunksize)) (`KismetMathLibrary.Conv_IntToDouble` (* _index_2 _chunksize)) (`KismetMathLibrary.Conv_IntToDouble` (* _index_3 _chunksize)))) "AlwaysSpawn" "OverrideRootScale" null null)))))

(fn `UserConstructionScript`)