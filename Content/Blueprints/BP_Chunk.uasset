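; BP_Chunk is an asteroid field chunk that scatters static mesh components through a box-shaped volume.
; Its construction script adds components in a loop driven by AsteroidPerChunk.
; RandomVector, bounded by Length, Height and Width, supplies location, rotation direction and scale alike, so scale grows with chunk dimensions.
; The AsteroidMeshes reference is unconnected, and the event graph has no active logic.
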(fn `RandomVector`
  (returns (RandomVector :type "Vector Structure"))
  (return (`KismetMathLibrary.MakeVector` (* (`self.length`) (`KismetMathLibrary.RandomFloat`)) (* (`self.height`) (`KismetMathLibrary.RandomFloat`)) (* (`self.width`) (`KismetMathLibrary.RandomFloat`)))))

(fn `UserConstructionScript`
  (for _ (range (+ (`self.asteroidPerChunk`) 1))
    (`AddComponent|NODE_AddStaticMeshComponent-2` :`RelativeTransform` (`KismetMathLibrary.MakeTransform` (`self.RandomVector`) (`KismetMathLibrary.Conv_VectorToRotator` (`self.RandomVector`)) (`self.RandomVector`)))))